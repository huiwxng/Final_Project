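; BP_Easy is a trigger actor that runs the easy mode wave of zombies and civilians when the first-person character overlaps its boxes.
; EasyBox and EasyBox1 start looping "Easy" timers on the first BP_SpawnZombies and BP_SpawnCivilians found.
; After separate delays, each branch replaces its loop with a one-shot timer and destroys the whole actor.
; Only the longer zombie branch prints the completion message, so the shorter civilian branch can destroy the actor first.
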(event OnComponentBeginOverlap(EasyBox)
  (params (OverlappedComponent :type Primitive%20Component%20Object%20Reference) (OtherActor :type Actor%20Object%20Reference) (OtherComp :type Primitive%20Component%20Object%20Reference) (OtherBodyIndex :type Integer) (bFromSweep :type Boolean) (SweepResult :type Hit%20Result%20Structure%20%28by%20ref%29))
  (Utilities|Casting|CastToFirstPersonCharacter OtherActor)
  (bind _outactors (Actor|GetAllActorsOfClass "/Game/Hui/BP_SpawnZombies.BP_SpawnZombies_C"))
  (Utilities|Time|SetTimerbyFunctionName (Utilities|Array|Get(acopy) _outactors) "Easy" 2.0 true)
  (Utilities|FlowControl|Delay 2e+01)
  (Development|PrintString "EASY MODE COMPLETED!" true true "(R=0.415855,G=1.000000,B=0.000000,A=1.000000)")
  (Utilities|Time|SetTimerbyFunctionName (Utilities|Array|Get(acopy) _outactors) "Easy" 2.0)
  (Actor|DestroyActor))

(event OnComponentBeginOverlap(EasyBox1)
  (params (OverlappedComponent :type Primitive%20Component%20Object%20Reference) (OtherActor :type Actor%20Object%20Reference) (OtherComp :type Primitive%20Component%20Object%20Reference) (OtherBodyIndex :type Integer) (bFromSweep :type Boolean) (SweepResult :type Hit%20Result%20Structure%20%28by%20ref%29))
  (Utilities|Casting|CastToFirstPersonCharacter OtherActor)
  (bind _outactors (Actor|GetAllActorsOfClass "/Game/Hui/BP_SpawnCivilians.BP_SpawnCivilians_C"))
  (Utilities|Time|SetTimerbyFunctionName (Utilities|Array|Get(acopy) _outactors) "Easy" 6.0 true)
  (Utilities|FlowControl|Delay 1e+01)
  (Utilities|Time|SetTimerbyFunctionName (Utilities|Array|Get(acopy) _outactors) "Easy" 2.0)
  (Actor|DestroyActor))

(event EventBeginPlay)

(event Collision|EventActorBeginOverlap
  (params (OtherActor :type Actor%20Object%20Reference)))

(event EventTick
  (params (DeltaSeconds :type Float%20%28single-precision%29)))

(fn ConstructionScript)