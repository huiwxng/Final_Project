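; BP_Zombies is a shootable zombie target that awards score when killed.
; Each overlap with a FirstPersonProjectile subtracts one point from Health.
; At zero or below, it destroys itself, prints a kill message and adds TargetScore to the FirstPersonGameMode through AddTargetPoints.
; It has no movement, AI or construction logic of its own in these graphs.
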(event EventBeginPlay
  (|CallParentFunction) ; This node is disabled and will not be called.\nDrag off pins to build functionality.
)

(event Collision|EventActorBeginOverlap
  (params (OtherActor :type Actor%20Object%20Reference))
  (Utilities|Casting|CastToFirstPersonProjectile OtherActor)
  (Variables|Default|SetHealth (- (Variables|Default|GetHealth) 1.0))
  (if (<= (Variables|Default|GetHealth) 0.0)
    (Actor|DestroyActor)
    (Development|PrintText "Zombie Killed!   +100")
    (bind _asfirst_person_game_mode (Utilities|Casting|CastToFirstPersonGameMode (Game|GetGameMode)))
    (Default|AddTargetPoints _asfirst_person_game_mode (Variables|Default|GetTarget%20Score))))

(event EventTick
  (params (DeltaSeconds :type Float%20%28single-precision%29))
  (|CallParentFunction DeltaSeconds) ; This node is disabled and will not be called.\nDrag off pins to build functionality.
)

(fn ConstructionScript
  (|CallParentFunction))