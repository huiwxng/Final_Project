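; BP_Medium is a trigger actor that runs Medium mode when the first-person character overlaps its boxes.
; EasyBox loops Medium on BP_SpawnZombies for 40 seconds, then prints completion, re-sets that timer as one-shot and destroys the actor.
; EasyBox1 loops Easy on BP_SpawnCivilians, then after 20 seconds sets a one-shot Medium timer, leaving Easy looping.
; That branch also destroys the actor, cutting off any pending zombie completion.
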(event OnComponentBeginOverlap(EasyBox)
  (params (OverlappedComponent :type Primitive%20Component%20Object%20Reference) (OtherActor :type Actor%20Object%20Reference) (OtherComp :type Primitive%20Component%20Object%20Reference) (OtherBodyIndex :type Integer) (bFromSweep :type Boolean) (SweepResult :type Hit%20Result%20Structure%20%28by%20ref%29))
  (Utilities|Casting|CastToFirstPersonCharacter OtherActor)
  (bind _outactors (Actor|GetAllActorsOfClass "/Game/Hui/BP_SpawnZombies.BP_SpawnZombies_C"))
  (Utilities|Time|SetTimerbyFunctionName (Utilities|Array|Get(acopy) _outactors) "Medium" 1.0 true)
  (Utilities|FlowControl|Delay 4e+01)
  (Development|PrintString "MEDIUM MODE COMPLETED!" true true "(R=1.000000,G=0.333932,B=0.000000,A=1.000000)")
  (Utilities|Time|SetTimerbyFunctionName (Utilities|Array|Get(acopy) _outactors) "Medium" 1.0)
  (Actor|DestroyActor))

(event OnComponentBeginOverlap(EasyBox1)
  (params (OverlappedComponent :type Primitive%20Component%20Object%20Reference) (OtherActor :type Actor%20Object%20Reference) (OtherComp :type Primitive%20Component%20Object%20Reference) (OtherBodyIndex :type Integer) (bFromSweep :type Boolean) (SweepResult :type Hit%20Result%20Structure%20%28by%20ref%29))
  (Utilities|Casting|CastToFirstPersonCharacter OtherActor)
  (bind _outactors (Actor|GetAllActorsOfClass "/Game/Hui/BP_SpawnCivilians.BP_SpawnCivilians_C"))
  (Utilities|Time|SetTimerbyFunctionName (Utilities|Array|Get(acopy) _outactors) "Easy" 3.0 true)
  (Utilities|FlowControl|Delay 2e+01)
  (Utilities|Time|SetTimerbyFunctionName (Utilities|Array|Get(acopy) _outactors) "Medium" 1.0)
  (Actor|DestroyActor))

(event EventBeginPlay)

(event Collision|EventActorBeginOverlap
  (params (OtherActor :type Actor%20Object%20Reference)))

(event EventTick
  (params (DeltaSeconds :type Float%20%28single-precision%29)))

(fn ConstructionScript)