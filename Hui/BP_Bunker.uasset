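; BP_Bunker is a bunker actor that scores zombies and civilians entering it.
; Two overlap boxes each react to one type: ZombieBox to BP_Zombies, CivilianBox to BP_Civilians, destroying the actor that enters.
; It then calls FirstPersonGameMode to subtract points for a zombie or add points for a civilian, using its own point variables, and prints a message.
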(event OnComponentBeginOverlap(ZombieBox)
  (params (OverlappedComponent :type Primitive%20Component%20Object%20Reference) (OtherActor :type Actor%20Object%20Reference) (OtherComp :type Primitive%20Component%20Object%20Reference) (OtherBodyIndex :type Integer) (bFromSweep :type Boolean) (SweepResult :type Hit%20Result%20Structure%20%28by%20ref%29))
  (bind _asbp_zombies (Utilities|Casting|CastToBP_Zombies OtherActor))
  (Actor|DestroyActor _asbp_zombies)
  (bind _asfirst_person_game_mode (Utilities|Casting|CastToFirstPersonGameMode (Game|GetGameMode)))
  (Default|SubtractTargetPoints _asfirst_person_game_mode (Variables|Default|GetZombie%20In%20Bunker))
  (Development|PrintText "ZOMBIE IN THE BUNKER!"))

(event OnComponentBeginOverlap(CivilianBox)
  (params (OverlappedComponent :type Primitive%20Component%20Object%20Reference) (OtherActor :type Actor%20Object%20Reference) (OtherComp :type Primitive%20Component%20Object%20Reference) (OtherBodyIndex :type Integer) (bFromSweep :type Boolean) (SweepResult :type Hit%20Result%20Structure%20%28by%20ref%29))
  (bind _asbp_civilians (Utilities|Casting|CastToBP_Civilians OtherActor))
  (Actor|DestroyActor _asbp_civilians)
  (bind _asfirst_person_game_mode (Utilities|Casting|CastToFirstPersonGameMode (Game|GetGameMode)))
  (Default|AddTargetPoints _asfirst_person_game_mode (Variables|Default|GetCivilian%20in%20Bunker))
  (Development|PrintText "Civilian made it into the bunker safely!"))

(event EventBeginPlay)

(event Collision|EventActorBeginOverlap
  (params (OtherActor :type Actor%20Object%20Reference)))

(event EventTick
  (params (DeltaSeconds :type Float%20%28single-precision%29)))

(fn ConstructionScript)