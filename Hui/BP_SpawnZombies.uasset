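; BP_SpawnZombies is a spawner that places BP_Zombies at random points inside its SpawnBox bounds and sends them toward the bunker.
; Easy, Medium and Hard events all run the same logic.
; Each call spawns one zombie only while fewer than 70 BP_Characters actors exist, then calls ToBunker on it.
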(event Custom|Easy
  (bind _spawnbox (Variables|Default|GetSpawnBox))
  (bind (_origin _boxextent) (Collision|GetComponentBounds _spawnbox))
  (bind _outactors (Actor|GetAllActorsOfClass "/Game/Hui/BP_Characters.BP_Characters_C"))
  (if (< (Utilities|Array|Length _outactors) 70)
    (bind _returnvalue (AI|SpawnAIFromClass "/Game/Hui/BP_Zombies.BP_Zombies_C" 0 (Math|Random|RandomPointinBoundingBox _origin _boxextent) "0, 0, 0" false))
    (bind _asbp_zombies (Utilities|Casting|CastToBP_Zombies _returnvalue))
    (Default|ToBunker _asbp_zombies)))

(event Custom|Medium
  (bind _spawnbox (Variables|Default|GetSpawnBox))
  (bind (_origin _boxextent) (Collision|GetComponentBounds _spawnbox))
  (bind _outactors (Actor|GetAllActorsOfClass "/Game/Hui/BP_Characters.BP_Characters_C"))
  (if (< (Utilities|Array|Length _outactors) 70)
    (bind _returnvalue (AI|SpawnAIFromClass "/Game/Hui/BP_Zombies.BP_Zombies_C" 0 (Math|Random|RandomPointinBoundingBox _origin _boxextent) "0, 0, 0" false))
    (bind _asbp_zombies (Utilities|Casting|CastToBP_Zombies _returnvalue))
    (Default|ToBunker _asbp_zombies)))

(event Custom|Hard
  (bind _spawnbox (Variables|Default|GetSpawnBox))
  (bind (_origin _boxextent) (Collision|GetComponentBounds _spawnbox))
  (bind _outactors (Actor|GetAllActorsOfClass "/Game/Hui/BP_Characters.BP_Characters_C"))
  (if (< (Utilities|Array|Length _outactors) 70)
    (bind _returnvalue (AI|SpawnAIFromClass "/Game/Hui/BP_Zombies.BP_Zombies_C" 0 (Math|Random|RandomPointinBoundingBox _origin _boxextent) "0, 0, 0" false))
    (bind _asbp_zombies (Utilities|Casting|CastToBP_Zombies _returnvalue))
    (Default|ToBunker _asbp_zombies)))

(fn ConstructionScript)