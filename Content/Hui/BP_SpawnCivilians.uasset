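; BP_SpawnCivilians spawns AI civilians at random points inside its SpawnBox and calls ToBunker on each.
; Each call spawns one BP_Civilians, provided fewer than 15 BP_Characters actors exist in the world.
; The Easy, Medium and Hard events all run this same logic, so difficulty currently makes no difference to spawning.
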(event Custom|Easy
  (bind _spawnbox (Variables|Default|GetSpawnBox))
  (bind (_origin _boxextent) (Collision|GetComponentBounds _spawnbox))
  (bind _outactors (Actor|GetAllActorsOfClass "/Game/Hui/BP_Characters.BP_Characters_C"))
  (if (< (Utilities|Array|Length _outactors) 15)
    (bind _returnvalue (AI|SpawnAIFromClass "/Game/Hui/BP_Civilians.BP_Civilians_C" 0 (Math|Random|RandomPointinBoundingBox _origin _boxextent) "0, 0, 0" false))
    (bind _asbp_civilians (Utilities|Casting|CastToBP_Civilians _returnvalue))
    (Default|ToBunker _asbp_civilians)))

(event Custom|Medium
  (bind _spawnbox (Variables|Default|GetSpawnBox))
  (bind (_origin _boxextent) (Collision|GetComponentBounds _spawnbox))
  (bind _outactors (Actor|GetAllActorsOfClass "/Game/Hui/BP_Characters.BP_Characters_C"))
  (if (< (Utilities|Array|Length _outactors) 15)
    (bind _returnvalue (AI|SpawnAIFromClass "/Game/Hui/BP_Civilians.BP_Civilians_C" 0 (Math|Random|RandomPointinBoundingBox _origin _boxextent) "0, 0, 0" false))
    (bind _asbp_civilians (Utilities|Casting|CastToBP_Civilians _returnvalue))
    (Default|ToBunker _asbp_civilians)))

(event Custom|Hard
  (bind _spawnbox (Variables|Default|GetSpawnBox))
  (bind (_origin _boxextent) (Collision|GetComponentBounds _spawnbox))
  (bind _outactors (Actor|GetAllActorsOfClass "/Game/Hui/BP_Characters.BP_Characters_C"))
  (if (< (Utilities|Array|Length _outactors) 15)
    (bind _returnvalue (AI|SpawnAIFromClass "/Game/Hui/BP_Civilians.BP_Civilians_C" 0 (Math|Random|RandomPointinBoundingBox _origin _boxextent) "0, 0, 0" false))
    (bind _asbp_civilians (Utilities|Casting|CastToBP_Civilians _returnvalue))
    (Default|ToBunker _asbp_civilians)))

(fn ConstructionScript)